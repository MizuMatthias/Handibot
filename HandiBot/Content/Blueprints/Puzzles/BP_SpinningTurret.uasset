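; Prototype puzzle turret that alternates between spinning and firing a laser, never both at once.
; A fast looping timer calls an event that branches on a temporary flag, standing in for a linked device's state, which Delays flip every few seconds.
; SPIND steps the yaw in small increments; SHOOT runs a debug-drawn forward sphere trace from the Arrow, with the hit result not yet used.
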(event `self.ReceiveBeginPlay`
  ;[0.2595 1 0.1295] Short timer ensures that the turret spins at a rapid and smooth rate
  (`KismetSystemLibrary.K2_SetTimerDelegate` (delegate `Spin? Or Shoot?`) 0.01 true true))

(event `Spin? Or Shoot?`
  ;[0.2595 1 0.1295] Is the designated device (amplink or complink on or off?
  (if (`self.tempVariable`)
    ;[0.2595 1 0.1295] The turret can only do one action at a time (cant spin and shoot at the same time) and so lasers must be timed accordingly
    (`self.SHOOT!  >:)`)
    ;[1 0.1551 0.1352] Temporary stuff to check everything works
    (`KismetSystemLibrary.Delay` 2.0)
    (set `self.tempVariable` false)
    (else
      (`self.SPIN!  :D`)
      (`KismetSystemLibrary.Delay` 4.0)
      (set `self.tempVariable` true))))

(fn `SHOOT!  >:)`
  (bind _arrow (`self.Arrow`))
  (bind _returnvalue (`SceneComponent.K2_GetComponentLocation` _arrow))
  ;[0.2595 1 0.1295] Shoot laser while not rotating. You can link it to some sort of target blueprint and open a door if it hits, or make it a killing machine. Depends on what you want to use this for
  (`KismetSystemLibrary.SphereTraceSingle` :`Start` _returnvalue :`End` (+ _returnvalue (* (`SceneComponent.GetForwardVector` _arrow) 800)) :`Radius` 15.0 :`TraceChannel` "TraceTypeQuery1" :`DrawDebugType` "ForDuration" :`TraceColor` (struct :`G` 1.0 :`B` 0.889245 :`A` 1.0) :`TraceHitColor` (struct :`R` 1.0 :`B` 0.979217 :`A` 1.0) :`DrawTime` 1.0))

(fn `SPIN!  :D`
  ;[0.2595 1 0.1295] Ensures that the turret rotates by a tiny amount every time the function is called.
  (bind _output_get (set `self.CurrentRotation` (+ (`self.CurrentRotation`) 2.0)))
  ;[0.2595 1 0.1295] R O T A T E
  (`self.K2_SetActorRotation` (`KismetMathLibrary.MakeRotator` 0.0 0.0 _output_get))
  ;[0.2595 1 0.1295] After the turret makes a complete rotation, set the variable back to 0 so nothing gets messed up
  (if (== (`self.CurrentRotation`) 360.0)
    (set `self.CurrentRotation` 0.0)))

(fn `UserConstructionScript`)