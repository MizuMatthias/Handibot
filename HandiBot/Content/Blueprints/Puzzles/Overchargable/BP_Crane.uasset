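; BP_Crane is a puzzle crane in the Overchargable folder that moves a generated CubeGrid mesh whenever its Toggle event fires.
; A FlipFlop alternately plays and reverses the Crane timeline.
; The timeline value drives StaticMesh1's Z scale while lowering and yawing the CubeGrid piece, so lengthening and descent stay in sync.
; Begin Overlap and Tick are disabled stubs, and construction only calls the parent.
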(event `self.Toggle`
  (`/Engine/EditorBlueprintResources/StandardMacros.FlipFlop`
    (:`A`
      (bind (_direction _value) (`Timeline|Crane` :!label _label)
        (:`Update`
          (`SceneComponent.SetRelativeScale3D` (`self.StaticMesh1`) (`KismetMathLibrary.MakeVector` 0.5 0.5 (+ (* _value 6.0) 6.0)))
          (`SceneComponent.K2_SetRelativeLocationAndRotation` (`self.CubeGridToolOutput_56B30638`) (`KismetMathLibrary.MakeVector` 100.0 1100.0 (- 1200.0 (* _value 1200.0))) (`KismetMathLibrary.MakeRotator` 0.0 0.0 (* _value -180.0)) false false))))
    (:`B`
      (goto _label :!via `Reverse`))))

(fn `UserConstructionScript`
  (`parent.UserConstructionScript`))