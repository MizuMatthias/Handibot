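; BP_MagnetParent is a puzzle actor, named as a parent for magnet objects, that triggers the Handibot player's magnet attachment.
; On BeginPlay it caches the player pawn as a BP_Handibot reference.
; When the player's right hand component begins overlapping Sphere1 while the right hand state is Magnet, it calls AttachMagnet on the player, leaving the attachment logic to the Handibot.
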(event `self.ReceiveBeginPlay`
  (bind _asbp_handibot (cast `/Game/Blueprints/Character/BP_Handibot` (`GameplayStatics.GetPlayerPawn` 0)))
  (set `self.Player REF` _asbp_handibot))

(event `self.Sphere1.OnComponentBeginOverlap`
  (params (OverlappedComponent :type "PrimitiveComponent Object Reference") (OtherActor :type "Actor Object Reference") (OtherComp :type "PrimitiveComponent Object Reference") (OtherBodyIndex :type Integer) (bFromSweep :type Boolean) (SweepResult :type "HitResult Structure (by ref)"))
  (bind _player_ref (`self.Player REF`))
  (if (== OtherComp (`/Game/Blueprints/Character/BP_Handibot.HandRight` _player_ref))
    (switch `/Game/Blueprints/Character/Enum_HandToolRight` (`/Game/Blueprints/Character/BP_Handibot.RightHandState` _player_ref)
      (:`NewEnumerator2`
        (`/Game/Blueprints/Character/BP_Handibot.AttachMagnet` (`self.Player REF`))))))

(fn `UserConstructionScript`)