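; BP_OverchargePanel is a puzzle socket that lets the player's Handibot toggle linked overchargeable actors.
; When the Handibot's box overlaps with its left hand in the required state, it registers as SocketComponent, previews the hand material, and shows a skeletal mesh with spark audio.
; Ending the overlap reverts these.
; Overcharge toggles each BP_OverchargableParent in ActorsToToggle with a sound; its Overcharged branch leaves the flag unchanged.
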(event `self.ReceiveBeginPlay`
  (bind _asbp_handibot (cast `/Game/Blueprints/Character/BP_Handibot` (`GameplayStatics.GetPlayerPawn` 0)))
  (set `self.Player REF` _asbp_handibot)
  (bind _returnvalue (`GameplayStatics.SpawnSound2D` "/Game/Sounds/amplink-electricity-sparks.amplink-electricity-sparks" 1.0 1.0 0.0 null))
  (`AudioComponent.SetPaused` _returnvalue true))

(event `self.Box.OnComponentBeginOverlap`
  (params (OverlappedComponent :type "PrimitiveComponent Object Reference") (OtherActor :type "Actor Object Reference") (OtherComp :type "PrimitiveComponent Object Reference") (OtherBodyIndex :type Integer) (bFromSweep :type Boolean) (SweepResult :type "HitResult Structure (by ref)"))
  (bind _player_ref (`self.Player REF`))
  (bind _player_ref_2 (`self.Player REF`))
  (if (and (== OtherComp (`/Game/Blueprints/Character/BP_Handibot.Box` _player_ref)) (`|EnumEquality` (`/Game/Blueprints/Character/BP_Handibot.LeftHandState` _player_ref) "NewEnumerator1"))
    (set `/Game/Blueprints/Character/BP_Handibot.SocketComponent` self _player_ref_2)
    (`PrimitiveComponent.SetMaterial` (`/Game/Blueprints/Character/BP_Handibot.HandLeft` _player_ref_2) 0 "/Engine/EditorResources/FieldNodes/_Resources/M_FieldRadiusPreview.M_FieldRadiusPreview")
    (`SceneComponent.SetVisibility` (`self.SkeletalMesh`) true false)
    (`AudioComponent.SetPaused` (stale `self.ReceiveBeginPlay` _returnvalue) false)))

(event `self.Box.OnComponentEndOverlap`
  (params (OverlappedComponent :type "PrimitiveComponent Object Reference") (OtherActor :type "Actor Object Reference") (OtherComp :type "PrimitiveComponent Object Reference") (OtherBodyIndex :type Integer))
  (bind _player_ref (`self.Player REF`))
  (if (== OtherComp (`/Game/Blueprints/Character/BP_Handibot.Box` (`self.Player REF`)))
    (set `/Game/Blueprints/Character/BP_Handibot.SocketComponent` null _player_ref)
    (`PrimitiveComponent.SetMaterial` (`/Game/Blueprints/Character/BP_Handibot.HandLeft` _player_ref) 0 "/Game/Materials/M_ShadedMaster.M_ShadedMaster")
    (`SceneComponent.SetVisibility` (`self.SkeletalMesh`) false false)
    (`AudioComponent.SetPaused` (stale `self.ReceiveBeginPlay` _returnvalue) true)))

(event `Overcharge`
  (if (`self.Overcharged?`)
    (set `self.Overcharged?` true)
    (else
      (set `self.Overcharged?` false)))
  (for _array_element (`self.ActorsToToggle`)
    (bind _asbp_overchargable_parent (cast `/Game/Blueprints/Puzzles/Overchargable/BP_OverchargableParent` _array_element))
    (`/Game/Blueprints/Puzzles/Overchargable/BP_OverchargableParent.Toggle` _asbp_overchargable_parent)
    (`GameplayStatics.PlaySound2D` "/Game/Sounds/overcharge-toggle_Cue.overcharge-toggle_Cue" 1.0 1.0 0.0 null null)))

(fn `UserConstructionScript`)