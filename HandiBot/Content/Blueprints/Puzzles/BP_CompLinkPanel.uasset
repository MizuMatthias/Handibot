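; BP_CompLinkPanel is a puzzle socket panel that lets the BP_Handibot player rotate a cylinder to drive linked actors.
; Box overlap with the player's box, gated on left-hand state, registers the panel as the SocketComponent, swaps the hand material and shows a skeletal mesh.
; UpdateRotate plays, reverses or stops the Rotation timeline, whose value turns the cylinder and feeds UpdateScaleValue on each BP_ComplinkableParent in ActorsToActivate.
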(event `self.ReceiveBeginPlay`
  (bind _asbp_handibot (cast `/Game/Blueprints/Character/BP_Handibot` (`GameplayStatics.GetPlayerPawn` 0)))
  (set `self.Player REF` _asbp_handibot))

(event `self.Box.OnComponentBeginOverlap`
  (params (OverlappedComponent :type "PrimitiveComponent Object Reference") (OtherActor :type "Actor Object Reference") (OtherComp :type "PrimitiveComponent Object Reference") (OtherBodyIndex :type Integer) (bFromSweep :type Boolean) (SweepResult :type "HitResult Structure (by ref)"))
  (bind _player_ref (`self.Player REF`))
  (bind _player_ref_2 (`self.Player REF`))
  (if (and (== OtherComp (`/Game/Blueprints/Character/BP_Handibot.Box` _player_ref)) (`|EnumEquality` (`/Game/Blueprints/Character/BP_Handibot.LeftHandState` _player_ref) "NewEnumerator2"))
    (set `/Game/Blueprints/Character/BP_Handibot.SocketComponent` self _player_ref_2)
    (`PrimitiveComponent.SetMaterial` (`/Game/Blueprints/Character/BP_Handibot.HandLeft` _player_ref_2) 0 "/Engine/EditorResources/FieldNodes/_Resources/M_FieldRadiusPreview.M_FieldRadiusPreview")
    (`SceneComponent.SetVisibility` (`self.SkeletalMesh`) true false)))

(event `self.Box.OnComponentEndOverlap`
  (params (OverlappedComponent :type "PrimitiveComponent Object Reference") (OtherActor :type "Actor Object Reference") (OtherComp :type "PrimitiveComponent Object Reference") (OtherBodyIndex :type Integer))
  (bind _player_ref (`self.Player REF`))
  (if (== OtherComp (`/Game/Blueprints/Character/BP_Handibot.Box` (`self.Player REF`)))
    (set `/Game/Blueprints/Character/BP_Handibot.SocketComponent` null _player_ref)
    (`PrimitiveComponent.SetMaterial` (`/Game/Blueprints/Character/BP_Handibot.HandLeft` _player_ref) 0 "/Game/Materials/M_ShadedMaster.M_ShadedMaster")
    (`SceneComponent.SetVisibility` (`self.SkeletalMesh`) false false)))

(event `UpdateRotate`
  (params (CW :type Boolean) (ACW :type Boolean))
  (if CW
    (if ACW
      (bind (_direction _rotationscale) (`Timeline|Rotation` :!via `Stop` :!label _label)
        (:`Update`
          (`SceneComponent.K2_SetRelativeRotation` (`self.Cylinder`) (`KismetMathLibrary.MakeRotator` 90.0 (* _rotationscale 360.0)) false false)
          (for _array_element (`self.ActorsToActivate`)
            (bind _asbp_complinkable_parent (cast `/Game/Blueprints/Puzzles/Complinkable/BP_ComplinkableParent` _array_element))
            (`/Game/Blueprints/Puzzles/Complinkable/BP_ComplinkableParent.UpdateScaleValue` _asbp_complinkable_parent _rotationscale))))
      (else
        (goto _label)))
    (elif ACW
      (goto _label :!via `Reverse`)
      (else
        (goto _label :!via `Stop`)))))

(fn `UserConstructionScript`)