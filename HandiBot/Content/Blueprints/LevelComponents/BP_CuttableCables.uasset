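; BP_CuttableCables is a level component: a bundle of cables that can be cut once its electricity is switched off.
; Toggle flips the electrified state, and while live a timeline periodically fires Niagara sparks at random rotations.
; CutDamage only applies when unpowered, detaching five cables one by one as hitpoints drop through thresholds.
; When hitpoints run out, the last cable detaches and the collision box stops blocking.
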(event `self.Toggle`
  (if (`self.isElectrified?`)
    (set `self.isElectrified?` false)
    (else
      (set `self.isElectrified?` true))))

(event `self.ReceiveBeginPlay`
  (bind _niagara (`self.Niagara`))
  (`Timeline|Spark Intervals` :!via `PlayFromStart`
    (:`Spark`
      (if (`self.isElectrified?`)
        (`SceneComponent.K2_SetRelativeRotation` _niagara (`KismetMathLibrary.MakeRotator` (`KismetMathLibrary.RandomFloatInRange` 0.0 360.0) (`KismetMathLibrary.RandomFloatInRange` 0.0 360.0) (`KismetMathLibrary.RandomFloatInRange` 0.0 360.0)) false false)
        (`ActorComponent.Activate` _niagara true)))))

(event `/Game/Blueprints/Interfaces/BPI_Cuttable.CutDamage`
  (params (`Damage Amount` :type "Float (double-precision)"))
  (if (not (`self.isElectrified?`))
    (bind _output_get (set `self.Hitpoints` (- (`self.Hitpoints`) `Damage Amount`)))
    (if (< _output_get 80.0)
      (set `CableComponent.bAttachEnd` false (`self.Cable1`))
      (if (< _output_get 60.0)
        (set `CableComponent.bAttachEnd` false (`self.Cable2`))
        (if (< _output_get 40.0)
          (set `CableComponent.bAttachEnd` false (`self.Cable3`))
          (if (< _output_get 20.0)
            (set `CableComponent.bAttachEnd` false (`self.Cable4`))
            (if (<= _output_get 0.0)
              (set `CableComponent.bAttachEnd` false (`self.Cable5`))
              (`PrimitiveComponent.SetCollisionEnabled` (`self.CollisionBox`) "NoCollision"))))))))

(fn `UserConstructionScript`)