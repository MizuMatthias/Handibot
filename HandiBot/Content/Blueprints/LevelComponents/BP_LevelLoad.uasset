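; BP_LevelLoad is a level entrance that opens its assigned level when BP_Handibot overlaps its E component.
; On BeginPlay it labels itself with its level number and, if NeedLevel1 is set, shows a Locked component while GI_Handibot reports level 1 incomplete.
; The overlap repeats that game instance check, so gated entrances open only after level 1 completion, while ungated ones open immediately.
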(event `self.ReceiveBeginPlay`
  (`TextRenderComponent.K2_SetText` (`self.Leveltext`) (`KismetTextLibrary.Conv_StringToText` (`KismetStringLibrary.Concat_StrStr` "Level: " (`KismetStringLibrary.Conv_IntToString` (`self.Level Number`)))))
  (if (`self.NeedLevel1?`)
    (bind _asgi_handibot (cast `/Game/Blueprints/Character/GI_Handibot` (`GameplayStatics.GetGameInstance`)))
    (if (not (`/Game/Blueprints/Character/GI_Handibot.CompleteLevel1?` _asgi_handibot))
      (`SceneComponent.SetVisibility` (`self.locked`) true false))
    (else
      (`SceneComponent.SetVisibility` (`self.locked`) false false))))

(event `self.e.OnComponentBeginOverlap`
  (params (OverlappedComponent :type "PrimitiveComponent Object Reference") (OtherActor :type "Actor Object Reference") (OtherComp :type "PrimitiveComponent Object Reference") (OtherBodyIndex :type Integer) (bFromSweep :type Boolean) (SweepResult :type "HitResult Structure (by ref)"))
  (cast `/Game/Blueprints/Character/BP_Handibot` OtherActor)
  (if (`self.NeedLevel1?`)
    (bind _asgi_handibot (cast `/Game/Blueprints/Character/GI_Handibot` (`GameplayStatics.GetGameInstance`)))
    (if (`/Game/Blueprints/Character/GI_Handibot.CompleteLevel1?` _asgi_handibot)
      (`GameplayStatics.OpenLevelBySoftObjectPtr` (`self.Level`) :!label _label))
    (else
      (goto _label))))

(fn `UserConstructionScript`)