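; BP_Enemy is an AI enemy that attacks the player's BP_Handibot, with looping-style engine and gibberish sounds attached to its mesh on spawn.
; PawnSensing stores the seen Handibot and sets the "CanSeePlayer?" blackboard key.
; Attack plays a Spin timeline that rotates the tilted mesh, with an event track damaging the Handibot at close range.
; CutDamage lowers Health with randomly rotated Niagara effects and sound, destroying the actor at zero.
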(event `self.ReceiveBeginPlay`
  (bind _staticmesh (`self.StaticMesh`))
  (`GameplayStatics.SpawnSoundAttached` "/Game/Sounds/engine.engine" _staticmesh "None" (0.0 0.0 0.0) (struct) "KeepRelativeOffset" false 0.5 1.0 0.0 "/Game/Sounds/Enemy_Att.Enemy_Att" null)
  (`GameplayStatics.SpawnSoundAttached` "/Game/Sounds/enemy-gibberish.enemy-gibberish" _staticmesh "None" (0.0 0.0 0.0) (struct) "KeepRelativeOffset" false 1.0 1.0 0.0 "/Game/Sounds/Enemy_Att.Enemy_Att" null))

(event `self.PawnSensing.OnSeePawn`
  (params (Pawn :type "Pawn Object Reference"))
  (bind _asbp_handibot (cast `/Game/Blueprints/Character/BP_Handibot` Pawn))
  (set `self.As BP Handibot` _asbp_handibot)
  (`BlackboardComponent.SetValueAsBool` (`AIBlueprintHelperLibrary.GetBlackboard` (`AIBlueprintHelperLibrary.GetAIController` self)) "CanSeePlayer?" true))

(event `Attack`
  (bind (_direction _newtrack_0) (`Timeline|Spin` :!via `PlayFromStart`)
    (:`Update`
      (`SceneComponent.K2_SetRelativeRotation` (`self.StaticMesh`) (`KismetMathLibrary.MakeRotator` 0.0 15.0 (* _newtrack_0 360.0)) false false))
    (:`Finished`
      (`SceneComponent.K2_SetRelativeRotation` :`self` (`self.StaticMesh`)))
    (:`NewTrack_1`
      (if (<= (`self.GetDistanceTo` (`self.As BP Handibot`)) 100.0)
        (`/Game/Blueprints/Character/BP_Handibot.Damage` (`self.As BP Handibot`) 10.0)))))

(event `/Game/Blueprints/Interfaces/BPI_Cuttable.CutDamage`
  (params (`Damage Amount` :type "Float (double-precision)"))
  (bind _niagara (`self.Niagara`))
  (`GameplayStatics.PlaySound2D` "/Game/Sounds/cutting-tool-hit-breakable-object_Cue.cutting-tool-hit-breakable-object_Cue" 1.0 1.0 0.0 null null)
  (set `self.health` (- (`self.health`) `Damage Amount`))
  (`SceneComponent.K2_SetRelativeRotation` _niagara (`KismetMathLibrary.MakeRotator` (`KismetMathLibrary.RandomFloatInRange` 0.0 360.0) (`KismetMathLibrary.RandomFloatInRange` 0.0 360.0) (`KismetMathLibrary.RandomFloatInRange` 0.0 360.0)) false false)
  (`ActorComponent.Activate` _niagara true)
  (if (<= (`self.health`) 0.0)
    (`self.K2_DestroyActor`)
    (`GameplayStatics.PlaySound2D` "/Game/Sounds/hand-mechanism-swap-1_Cue.hand-mechanism-swap-1_Cue" 0.5 1.0 2.4 null null)))

(fn `UserConstructionScript`)